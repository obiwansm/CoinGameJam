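; Test actor for a dissolve VFX that dissolves its Cube and destroys itself when Archer_BP overlaps its Sphere.
; BeginPlay creates a dynamic material instance on the Cube from a referenced material.
; On overlap, the DissolveCurve timeline drives dissolve, fringe and glow intensity, with multipliers on the latter two.
; SetParameters pushes these plus surface, texture and color settings to the material every update, and the timeline's end destroys the actor.
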(event OnComponentBeginOverlap(Sphere)
  (params (OverlappedComponent :type Primitive%20Component%20Object%20Reference) (OtherActor :type Actor%20Object%20Reference) (OtherComp :type Primitive%20Component%20Object%20Reference) (OtherBodyIndex :type Integer) (bFromSweep :type Boolean) (SweepResult :type Hit%20Result%20Structure%20%28by%20ref%29))
  (Utilities|Casting|CastToArcher_BP OtherActor)
  (CallFunction|PlayDissolveAnimation))

(event Custom|Set%20Material%20instance
  (bind _returnvalue (Rendering|Material|CreateDynamicMaterialInstance (Variables|Default|GetCube) 0 (Variables|Default|GetMaterial%20Reference) "None" :!class /Script/Engine.PrimitiveComponent))
  (Variables|Default|SetMaterial%20Instance%20Reference _returnvalue))

(event Custom|Play%20Dissolve%20Animation
  (bind (_direction _dissolve_amount_curve _fring_curve _emissive_curve) (Timeline|DissolveCurve Play)
    (:Update
      (CallFunction|SetParameters (Variables|Default|GetMaterial%20Instance%20Reference) _dissolve_amount_curve (* _fring_curve (Variables|Default|GetFringeMulti)) (* _emissive_curve (Variables|Default|GetEmissiveMulti)) (Variables|Default|GetScale%20Value) (Variables|Default|GetMetallicValue) (Variables|Default|GetSpecularValue) (Variables|Default|GetRoughnessValue) (Variables|Default|GetColor%20Texture%20Reference) (Variables|Default|GetDissolveMask) (Variables|Default|GetColor%20Glow)))
    (:Finished
      (Actor|DestroyActor))))

(event EventBeginPlay
  (CallFunction|SetMaterialInstance))

(fn ConstructionScript)

(fn SetParameters
  (params (Target%20Material :type Material%20Instance%20Dynamic%20Object%20Reference) (Dissolve%20Amount :type Float%20%28single-precision%29) (Fringe :type Float%20%28single-precision%29) (Emissive%20Amount :type Float%20%28single-precision%29) (Texture%20Scale :type Float%20%28single-precision%29) (Metallic :type Float%20%28single-precision%29) (Specular :type Float%20%28single-precision%29) (Roughness :type Float%20%28single-precision%29) (Color%20Texture :type Texture%20Object%20Reference) (Dissolve%20Mask :type Texture%20Object%20Reference) (Glow%20Color :type Linear%20Color%20Structure))
  (Rendering|Material|SetScalarParameterValue Target%20Material (Variables|Default|GetDissolve%20Amount) Dissolve%20Amount :!class /Script/Engine.MaterialInstanceDynamic)
  (Rendering|Material|SetScalarParameterValue Target%20Material (Variables|Default|GetFringe) Fringe :!class /Script/Engine.MaterialInstanceDynamic)
  (Rendering|Material|SetScalarParameterValue Target%20Material (Variables|Default|GetEmissive%20Amount) Emissive%20Amount :!class /Script/Engine.MaterialInstanceDynamic)
  (Rendering|Material|SetScalarParameterValue Target%20Material (Variables|Default|GetTextureScale) Texture%20Scale :!class /Script/Engine.MaterialInstanceDynamic)
  (Rendering|Material|SetScalarParameterValue Target%20Material (Variables|Default|GetMetallic) Metallic :!class /Script/Engine.MaterialInstanceDynamic)
  (Rendering|Material|SetScalarParameterValue Target%20Material (Variables|Default|GetSpecular) Specular :!class /Script/Engine.MaterialInstanceDynamic)
  (Rendering|Material|SetScalarParameterValue Target%20Material (Variables|Default|GetRoughness) Roughness :!class /Script/Engine.MaterialInstanceDynamic)
  (Rendering|Material|SetTextureParameterValue Target%20Material (Variables|Default|GetColor%20Texture) Color%20Texture)
  (Rendering|Material|SetTextureParameterValue Target%20Material (Variables|Default|GetDissolve%20Mask) Dissolve%20Mask)
  (Rendering|Material|SetVectorParameterValue Target%20Material (Variables|Default|GetGlow%20Color) Glow%20Color :!class /Script/Engine.MaterialInstanceDynamic))