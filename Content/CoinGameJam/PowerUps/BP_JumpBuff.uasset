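; BP_JumpBuff is a power-up that boosts the player's jump at the cost of their ability to dodge.
; AddBuff sets the JumpBuff flag, multiplies jump velocity by JumpMultiplier and prints an on-screen notice for BuffDuration, while AddDebuff disables dodging.
; RemoveBuff and RemoveDebuff undo these effects, restoring jump velocity to a hardcoded value rather than the player's previous one.
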(event EventAddDebuff
  (params (PlayerRef :type Archer%20BP%20Object%20Reference))
  (Variables|/Game/CoinGameJam/PersonagemPrincipal/Blueprints/Archer_BP.Archer_BP_C|SetbCanDodge PlayerRef false))

(event EventRemoveBuff
  (params (PlayerRef :type Archer%20BP%20Object%20Reference))
  (Variables|/Game/CoinGameJam/PersonagemPrincipal/Blueprints/Archer_BP.Archer_BP_C|SetbJumpBuff PlayerRef false)
  (Variables|/Script/Engine.CharacterMovementComponent|SetJumpZVelocity (Variables|/Script/Engine.Character|GetCharacterMovement PlayerRef) 8e+02))

(event EventRemoveDebuff
  (params (PlayerRef :type Archer%20BP%20Object%20Reference))
  (Variables|/Game/CoinGameJam/PersonagemPrincipal/Blueprints/Archer_BP.Archer_BP_C|SetbCanDodge PlayerRef true))

(event EventAddBuff
  (params (PlayerRef :type Archer%20BP%20Object%20Reference))
  (bind _charactermovement (Variables|/Script/Engine.Character|GetCharacterMovement PlayerRef))
  (Variables|/Game/CoinGameJam/PersonagemPrincipal/Blueprints/Archer_BP.Archer_BP_C|SetbJumpBuff PlayerRef true)
  (Variables|/Script/Engine.CharacterMovementComponent|SetJumpZVelocity _charactermovement (* (Variables|/Script/Engine.CharacterMovementComponent|GetJumpZVelocity _charactermovement) (Variables|Default|GetjumpMultiplier)))
  (Development|PrintString (Utilities|String|Append "Jump x1.5" " / " "Can't Dodge") true true "(R=0.000000,G=0.660000,B=1.000000,A=1.000000)" (Variables|Default|GetbuffDuration)))

(fn ConstructionScript
  (|CallParentFunction))