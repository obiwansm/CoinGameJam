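; BP_BaseBuff is a base power-up pickup that applies a timed buff and debuff to the Archer_BP character that overlaps its sphere.
; On overlap it calls AddBuff and AddDebuff, hides itself and disables collision, then after BuffDuration calls the matching Remove functions and destroys itself.
; The four buff functions are empty hooks, presumably for child classes to override.
; Tick spins the pickup continuously around its yaw axis.
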(event OnComponentBeginOverlap(Sphere)
  (params (OverlappedComponent :type Primitive%20Component%20Object%20Reference) (OtherActor :type Actor%20Object%20Reference) (OtherComp :type Primitive%20Component%20Object%20Reference) (OtherBodyIndex :type Integer) (bFromSweep :type Boolean) (SweepResult :type Hit%20Result%20Structure%20%28by%20ref%29))
  (bind _asarcher_bp (Utilities|Casting|CastToArcher_BP OtherActor))
  (CallFunction|AddBuff _asarcher_bp)
  (CallFunction|AddDebuff _asarcher_bp)
  (Rendering|SetActorHiddenInGame true)
  (Collision|SetCollisionEnabled (Variables|Default|GetSphere) "NoCollision")
  (Utilities|FlowControl|Delay (Variables|Default|GetbuffDuration))
  (CallFunction|RemoveBuff _asarcher_bp)
  (CallFunction|RemoveDebuff _asarcher_bp)
  (Actor|DestroyActor)
  (Development|PrintString "BuffDestroy"))

(event EventTick
  (params (DeltaSeconds :type Float%20%28single-precision%29))
  (Transformation|AddActorLocalRotation (Math|Rotator|MakeRotator 0.0 0.0 (* DeltaSeconds 3e+02)) false false))

(fn ConstructionScript)

(fn AddBuff
  (params (PlayerRef :type Archer%20BP%20Object%20Reference)))

(fn AddDebuff
  (params (PlayerRef :type Archer%20BP%20Object%20Reference)))

(fn RemoveBuff
  (params (PlayerRef :type Archer%20BP%20Object%20Reference)))

(fn RemoveDebuff
  (params (PlayerRef :type Archer%20BP%20Object%20Reference)))