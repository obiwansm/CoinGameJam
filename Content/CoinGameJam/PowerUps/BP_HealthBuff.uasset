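; BP_HealthBuff is a power-up that grants the player health regeneration at the cost of reduced movement speed and damage.
; It implements add and remove events for the buff, which toggles the player's HealthBuff flag, and for the debuff, which scales base damage and sets the target speed multiplier.
; Removal divides damage back and resets speed to normal.
; Applying the buff prints a hardcoded effect summary on screen for the buff's duration.
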(event EventAddDebuff
  (params (PlayerRef :type Archer%20BP%20Object%20Reference))
  (Variables|/Game/CoinGameJam/PersonagemPrincipal/Blueprints/Archer_BP.Archer_BP_C|SetbaseDamage PlayerRef (* (Variables|/Game/CoinGameJam/PersonagemPrincipal/Blueprints/Archer_BP.Archer_BP_C|GetbaseDamage PlayerRef) (Variables|Default|GetdamageMultiplier)))
  (Variables|/Game/CoinGameJam/PersonagemPrincipal/Blueprints/Archer_BP.Archer_BP_C|SettargetSpeedMultiplier PlayerRef (Variables|Default|GetspeedMultiplier)))

(event EventRemoveBuff
  (params (PlayerRef :type Archer%20BP%20Object%20Reference))
  (Variables|/Game/CoinGameJam/PersonagemPrincipal/Blueprints/Archer_BP.Archer_BP_C|SetbHealthBuff PlayerRef false))

(event EventRemoveDebuff
  (params (PlayerRef :type Archer%20BP%20Object%20Reference))
  (Variables|/Game/CoinGameJam/PersonagemPrincipal/Blueprints/Archer_BP.Archer_BP_C|SetbaseDamage PlayerRef (/ (Variables|/Game/CoinGameJam/PersonagemPrincipal/Blueprints/Archer_BP.Archer_BP_C|GetbaseDamage PlayerRef) (Variables|Default|GetdamageMultiplier)))
  (Variables|/Game/CoinGameJam/PersonagemPrincipal/Blueprints/Archer_BP.Archer_BP_C|SettargetSpeedMultiplier PlayerRef 1.0))

(event EventAddBuff
  (params (PlayerRef :type Archer%20BP%20Object%20Reference))
  (Variables|/Game/CoinGameJam/PersonagemPrincipal/Blueprints/Archer_BP.Archer_BP_C|SetbHealthBuff PlayerRef true)
  (Development|PrintString (Utilities|String|Append "Health Regen" " / " "Speed x0.8" " / " "Damage x0.8") true true "(R=0.000000,G=0.660000,B=1.000000,A=1.000000)" (Variables|Default|GetbuffDuration)))

(fn ConstructionScript
  (|CallParentFunction))