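; BP_DamageBuff is a power-up that trades player movement speed for damage.
; AddBuff sets the player's DamageBuff flag, changes the target speed multiplier and prints a hardcoded effect message for the buff's duration.
; AddDebuff, despite its name, applies the damage multiplier to BaseDamage.
; RemoveBuff clears the flag and resets speed to normal, while RemoveDebuff divides the damage multiplier back out.
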(event EventAddDebuff
  (params (PlayerRef :type Archer%20BP%20Object%20Reference))
  (Variables|/Game/CoinGameJam/PersonagemPrincipal/Blueprints/Archer_BP.Archer_BP_C|SetbaseDamage PlayerRef (* (Variables|/Game/CoinGameJam/PersonagemPrincipal/Blueprints/Archer_BP.Archer_BP_C|GetbaseDamage PlayerRef) (Variables|Default|GetdamageMultiplier))))

(event EventRemoveBuff
  (params (PlayerRef :type Archer%20BP%20Object%20Reference))
  (Variables|/Game/CoinGameJam/PersonagemPrincipal/Blueprints/Archer_BP.Archer_BP_C|SetbDamageBuff PlayerRef false)
  (Variables|/Game/CoinGameJam/PersonagemPrincipal/Blueprints/Archer_BP.Archer_BP_C|SettargetSpeedMultiplier PlayerRef 1.0))

(event EventRemoveDebuff
  (params (PlayerRef :type Archer%20BP%20Object%20Reference))
  (Variables|/Game/CoinGameJam/PersonagemPrincipal/Blueprints/Archer_BP.Archer_BP_C|SetbaseDamage PlayerRef (/ (Variables|/Game/CoinGameJam/PersonagemPrincipal/Blueprints/Archer_BP.Archer_BP_C|GetbaseDamage PlayerRef) (Variables|Default|GetdamageMultiplier))))

(event EventAddBuff
  (params (PlayerRef :type Archer%20BP%20Object%20Reference))
  (Variables|/Game/CoinGameJam/PersonagemPrincipal/Blueprints/Archer_BP.Archer_BP_C|SetbDamageBuff PlayerRef true)
  (Variables|/Game/CoinGameJam/PersonagemPrincipal/Blueprints/Archer_BP.Archer_BP_C|SettargetSpeedMultiplier PlayerRef (Variables|Default|GetspeedMultiplier))
  (Development|PrintString (Utilities|String|Append "Damage x2.5" " / " "Speed x0.6") true true "(R=0.000000,G=0.660000,B=1.000000,A=1.000000)" (Variables|Default|GetbuffDuration)))

(fn ConstructionScript
  (|CallParentFunction))