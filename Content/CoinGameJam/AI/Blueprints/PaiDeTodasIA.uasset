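; PaiDeTodasIA is a base Blueprint for AI in CoinGameJam, its name meaning "father of all AI", that provides shared health and death handling.
; The construction script sets current health to max health.
; TookDamage subtracts damage when CanTakeDamage is true and calls Death once health drops below one.
; Death is an empty event here, apparently left for child Blueprints to define.
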(event Custom|TookDamage
  (params (damage :type Float%20%28single-precision%29))
  (if (Variables|Default|GetbCanTakeDamage)
    (Variables|Default|SetcurrentHealth (- (Variables|Default|GetcurrentHealth) damage))
    (if (< (Variables|Default|GetcurrentHealth) 1.0)
      (CallFunction|Death))))

(event Custom|Death)

(fn ConstructionScript
  (Variables|Default|SetcurrentHealth (Variables|Default|GetmaxHealth)))