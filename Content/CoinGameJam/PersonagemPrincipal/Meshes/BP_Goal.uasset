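; BP_Goal is a goal target that ends the game in victory when an Arrow_BP overlaps its Box.
; It caches all BP_AI actors at BeginPlay and calls Death on each still-valid one when hit.
; A 3-second Delay inside that loop leads to disabling Archer_BP input, clearing widgets and showing WG_VictoryUI, so victory requires at least one valid enemy.
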(event OnComponentBeginOverlap(Box)
  (params (OverlappedComponent :type Primitive%20Component%20Object%20Reference) (OtherActor :type Actor%20Object%20Reference) (OtherComp :type Primitive%20Component%20Object%20Reference) (OtherBodyIndex :type Integer) (bFromSweep :type Boolean) (SweepResult :type Hit%20Result%20Structure%20%28by%20ref%29))
  (bind _returnvalue (Game|GetPlayerController 0))
  (Utilities|Casting|CastToArrow_BP OtherActor)
  (for _array_element (Variables|Default|GetEnemies)
    (Utilities|IsValid _array_element
      (:Is%20Valid
        (Default|Death _array_element)
        (Utilities|FlowControl|Delay 3.0)
        (bind _asarcher_bp (Utilities|Casting|CastToArcher_BP (Game|GetPlayerCharacter 0)))
        (Input|DisableInput _asarcher_bp _returnvalue)
        (Viewport|RemoveAllWidgets)
        (bind _returnvalue_2 (UserInterface|CreateWidget "/Game/CoinGameJam/PersonagemPrincipal/UI/WG_VictoryUI.WG_VictoryUI_C" _returnvalue))
        (UserInterface|Viewport|AddtoViewport _returnvalue_2 0)))))

(event EventBeginPlay
  (bind _outactors (Actor|GetAllActorsOfClass "/Game/CoinGameJam/AI/Blueprints/BP_AI.BP_AI_C"))
  (Variables|Default|SetEnemies _outactors))

(event Collision|EventActorBeginOverlap
  (params (OtherActor :type Actor%20Object%20Reference)))

(event EventTick
  (params (DeltaSeconds :type Float%20%28single-precision%29)))

(fn ConstructionScript)