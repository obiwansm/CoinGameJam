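; Player archer character for a side-scrolling game, with jump, ground and air bow attacks, sprint and dodge roll.
; Holding Run/Dodge sprints; tapping rolls with input disabled until a montage notify.
; Attacks spawn arrows after a delay on the ground or on a notify in air.
; Tick interpolates facing and a look-ahead camera with a height floor and applies buff healing; BeginPlay creates the stats HUD.
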(event Custom|StartSprinting
  (if (Variables|Movement|GetbSprintPressed)
    (Variables|Movement|SettargetSpeed (Variables|Movement|GetsprintSpeed))
    (Variables|Movement|SetbSprinting true)))

(event EventBeginPlay
  (bind _returnvalue (UserInterface|CreateWidget "/Game/CoinGameJam/PersonagemPrincipal/UI/WG_CharacterStats.WG_CharacterStats_C" (Game|GetPlayerController 0)))
  (UserInterface|Viewport|AddtoViewport _returnvalue 0))

(event EventTick
  (params (DeltaSeconds :type Float%20%28single-precision%29))
  (|RotationControl)
  (|CameraControl)
  (if (Variables|Buffs|GetbHealthBuff)
    (Variables|Default|SetcurrentHealth (Math|Float|Clamp(Float) (+ (Variables|Default|GetcurrentHealth) 0.1) 0.0 (Variables|Default|GetmaxHealth)))))

(event Input|ActionEvents|InputActionJump
  (params (Key :type Key%20Structure))
  ;[1 1 1] Pulo simples
  (:Pressed
    (if (not (AI|Components|NavMovement|IsFalling (Variables|Character|GetCharacterMovement)))
      (Character|Jump))))

(event Input|ActionEvents|InputActionAttack
  (params (Key :type Key%20Structure))
  (:Pressed
    (if (not (Variables|Input|GetIsShooting?))
      (Audio|PlaySound2D "/Game/CoinGameJam/Sounds/SOMFlecha.SOMFlecha" 1.0 1.0 0.0 0 0)
      (if (AI|Components|NavMovement|IsFalling (Variables|Character|GetCharacterMovement))
        (bind _notifyname (Animation|Montage|PlayMontage (Variables|Character|GetMesh) "/Game/CoinGameJam/PersonagemPrincipal/Animations/Montages/AM_JumpAttack.AM_JumpAttack")
          (:then
            (Variables|Input|SetIsShooting? true))
          (:OnNotifyBegin
            (if (Utilities|Name|Equal(Name) _notifyname "JAttack")
              (Game|SpawnActorfromClass "/Game/CoinGameJam/PersonagemPrincipal/Blueprints/Arrow_BP.Arrow_BP_C" (Transformation|GetWorldTransform (Variables|Default|GetJumpAttackArrow)) "AdjustIfPossibleButAlwaysSpawn" 0 0)
              (Variables|Input|SetIsShooting? false))))
        (else
          (Animation|Montage|MontagePlay (Components|SkeletalMesh|GetAnimInstance (Variables|Character|GetMesh)) "/Game/CoinGameJam/PersonagemPrincipal/Animations/Montages/AM_Attack.AM_Attack" 1.0 "MontageLength" 0.0 true)
          (Variables|Input|SetIsShooting? true)
          (Utilities|FlowControl|Delay 0.316)
          (if true
            (Game|SpawnActorfromClass "/Game/CoinGameJam/PersonagemPrincipal/Blueprints/Arrow_BP.Arrow_BP_C" (Transformation|GetWorldTransform (Variables|Default|GetAttackArrow)) "AdjustIfPossibleButAlwaysSpawn" 0 0)
            (Variables|Input|SetIsShooting? false)))))))

(event Input|ActionEvents|InputActionRun/Dodge
  (params (Key :type Key%20Structure))
  (:Pressed
    (Variables|Movement|SetbSprintPressed true)
    (Utilities|Time|SetTimerbyEvent (delegate Custom|StartSprinting) 0.2))
  (:Released
    (Variables|Movement|SetbSprintPressed false)
    (if (Variables|Movement|GetbSprinting)
      (Variables|Movement|SettargetSpeed (Variables|Movement|GetjogSpeed))
      (Variables|Movement|SetbSprinting false)
      (elif (not (AI|Components|NavMovement|IsFalling (Variables|Character|GetCharacterMovement)))
        (Variables|Movement|SetbDodging true)
        (Input|DisableInput (Game|GetPlayerController 0))
        (bind _notifyname (Animation|Montage|PlayMontage (Variables|Character|GetMesh) "/Game/CoinGameJam/PersonagemPrincipal/Animations/Montages/Roll_Bow_RMAnim_Montage.Roll_Bow_RMAnim_Montage")
          (:OnNotifyBegin
            (if (Utilities|Name|Equal(Name) _notifyname "EnableInput")
              (Variables|Movement|SetbDodging false)
              (Input|EnableInput (Game|GetPlayerController 0)))))))))

(event Input|AxisEvents|InputAxisMoveForward/Backwards
  (params (AxisValue :type Float%20%28single-precision%29))
  ;[1 1 1] Movimento Simples
  (CallFunction|Movement AxisValue))

(fn ConstructionScript)

(fn Movement
  (params (movementInput :type Float%20%28single-precision%29))
  (bind _output_get (Variables|Input|SetmovementInput movementInput))
  (Variables|/Script/Engine.CharacterMovementComponent|SetMaxWalkSpeed (Variables|Character|GetCharacterMovement) (Math|Interpolation|FInterpTo (Variables|/Script/Engine.CharacterMovementComponent|GetMaxWalkSpeed (Variables|Character|GetCharacterMovement)) (* (Variables|Movement|GettargetSpeed) (Variables|Default|GettargetSpeedMultiplier)) (Utilities|Time|GetWorldDeltaSeconds) (* (Math|Float|Absolute(Float) (Variables|Input|GetmovementInput)) 2.0)))
  (Pawn|Input|AddMovementInput "1.000000, 0, 0" _output_get false))