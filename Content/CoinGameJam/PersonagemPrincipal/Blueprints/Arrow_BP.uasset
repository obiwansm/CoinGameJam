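; Arrow projectile that the player's Archer_BP damage stat powers, used to hurt BP_AI characters.
; On spawn it copies the archer's BaseDamage, launches its capsule with a forward physics impulse and destroys itself after a short lifetime.
; Overlapping a BP_AI applies that damage and removes the arrow, while a blocking hit swaps it for a StaticArrow_BP left at the impact location and rotation.
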(event OnComponentBeginOverlap(Capsule)
  (params (OverlappedComponent :type Primitive%20Component%20Object%20Reference) (OtherActor :type Actor%20Object%20Reference) (OtherComp :type Primitive%20Component%20Object%20Reference) (OtherBodyIndex :type Integer) (bFromSweep :type Boolean) (SweepResult :type Hit%20Result%20Structure%20%28by%20ref%29))
  (bind _asbp_ai (Utilities|Casting|CastToBP_AI OtherActor))
  (Default|TookDamage _asbp_ai (Variables|Default|GetarrowDamage))
  (Actor|DestroyActor))

(event OnComponentHit(Capsule)
  (params (HitComponent :type Primitive%20Component%20Object%20Reference) (OtherActor :type Actor%20Object%20Reference) (OtherComp :type Primitive%20Component%20Object%20Reference) (NormalImpulse :type Vector :default "0, 0, 0") (Hit :type Hit%20Result%20Structure%20%28by%20ref%29))
  (Game|SpawnActorfromClass "/Game/CoinGameJam/PersonagemPrincipal/Blueprints/StaticArrow_BP.StaticArrow_BP_C" (Math|Transform|MakeTransform (Transformation|GetWorldLocation (Variables|Default|GetCapsule)) (Transformation|GetWorldRotation (Variables|Default|GetArrow1)) "1,1,1") "AlwaysSpawn" 0 0)
  (Actor|DestroyActor))

(event EventBeginPlay
  (Collision|IgnoreActorwhenMoving (Variables|Default|GetCapsule) self true)
  (bind _asarcher_bp (Utilities|Casting|CastToArcher_BP (Game|GetPlayerCharacter 0)))
  (Variables|Default|SetarrowDamage (Variables|/Game/CoinGameJam/PersonagemPrincipal/Blueprints/Archer_BP.Archer_BP_C|GetbaseDamage _asarcher_bp))
  (Physics|AddImpulse (Variables|Default|GetCapsule) (* (Math|Vector|GetForwardVector (Variables|Default|GetArrow1)) 20000) "None" false)
  (Utilities|FlowControl|Delay 3.0)
  (Actor|DestroyActor))

(fn ConstructionScript)