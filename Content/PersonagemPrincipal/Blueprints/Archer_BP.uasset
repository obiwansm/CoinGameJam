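; Player archer character for side-scrolling movement along world X, with a launch-based jump and an airborne arrow attack.
; Jump launches upward without a ground check; Attack, only while falling, plays a sound, spawns Arrow_BP at JumpAttackArrow and calls a montage.
; Each tick, RotationControl derives facing from movement input and interpolates capsule yaw to turn the character.
; CameraControl then eases the camera boom's X offset toward the facing side.
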(event EventTick
  (params (DeltaSeconds :type Float%20%28single-precision%29))
  (|RotationControl)
  (|CameraControl))

(event Input|ActionEvents|InputActionJump
  (params (Key :type Key%20Structure))
  ;[1 1 1] Pulo simples
  (:Pressed
    (Character|LaunchCharacter "0, 0,1000.000000" false false)))

(event Input|ActionEvents|InputActionAttack
  (params (Key :type Key%20Structure))
  (:Pressed
    (if (AI|Components|NavMovement|IsFalling (Variables|Character|GetCharacterMovement))
      (Audio|PlaySound2D "/Game/Sounds/SOMFlecha.SOMFlecha" 1.0 1.0 0.0 0 0)
      (Game|SpawnActorfromClass "/Game/PersonagemPrincipal/Blueprints/Arrow_BP.Arrow_BP_C" (Transformation|GetWorldTransform (Variables|Default|GetJumpAttackArrow)) "Undefined" 0 0)
      (Animation|PlayAnimMontage 0 1.0 "None"))))

(event Input|AxisEvents|InputAxisMoveForward/Backwards
  (params (AxisValue :type Float%20%28single-precision%29))
  ;[1 1 1] Movimento Simples
  (bind _output_get (Variables|Default|SetmovementInput AxisValue))
  (Pawn|Input|AddMovementInput "1.000000, 0, 0" _output_get false))

(fn ConstructionScript)